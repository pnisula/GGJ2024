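; BP_NPC is a talkable character that picks its current dialogue from a DialogueManager actor based on story progress.
; On begin play it selects that character's dialogue list by CharacterID, then takes the first entry matching the GameInstance's saved dialogue ID and current day range.
; A box overlap registers the NPC as the player's CurrentNPC and toggles a custom-depth highlight.
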(event OnComponentBeginOverlap(Box)
  (params (OverlappedComponent :type Primitive%20Component%20Object%20Reference) (OtherActor :type Actor%20Object%20Reference) (OtherComp :type Primitive%20Component%20Object%20Reference) (OtherBodyIndex :type Integer) (bFromSweep :type Boolean) (SweepResult :type Hit%20Result%20Structure%20%28by%20ref%29))
  (bind _asbp_player_character (Utilities|Casting|CastToBP_PlayerCharacter OtherActor))
  (Variables|/Game/Blueprints/BP_PlayerCharacter.BP_PlayerCharacter_C|SetCurrent_NPC _asbp_player_character self)
  (Rendering|SetRenderCustomDepth (Variables|SkeletalMeshActor|GetSkeletalMeshComponent) true))

(event OnComponentEndOverlap(Box)
  (params (OverlappedComponent :type Primitive%20Component%20Object%20Reference) (OtherActor :type Actor%20Object%20Reference) (OtherComp :type Primitive%20Component%20Object%20Reference) (OtherBodyIndex :type Integer))
  (bind _asbp_player_character (Utilities|Casting|CastToBP_PlayerCharacter OtherActor))
  (Variables|/Game/Blueprints/BP_PlayerCharacter.BP_PlayerCharacter_C|SetCurrent_NPC _asbp_player_character 0)
  (Rendering|SetRenderCustomDepth (Variables|SkeletalMeshActor|GetSkeletalMeshComponent) false))

(event Custom|LoadDialogue
  (bind _dialoguemanager (Variables|Default|GetDialogueManager))
  (bind _characterid (Variables|Default|GetCharacterID))
  (Development|PrintString (Utilities|String|Append "Load new dialogue for: " (Utilities|String|ToString(Integer) _characterid)) true true "(R=0.000000,G=0.660000,B=1.000000,A=1.000000)" 1e+01)
  (switch int _characterid
    (:1
      (Variables|Default|SetNpcDialogues (Variables|/Game/Blueprints/Dialogue/DialogueManager.DialogueManager_C|GetNpc1Dialogues _dialoguemanager)))
    (:2
      (Variables|Default|SetNpcDialogues (Variables|/Game/Blueprints/Dialogue/DialogueManager.DialogueManager_C|GetNpc2Dialogues _dialoguemanager)))
    (:3
      (Variables|Default|SetNpcDialogues (Variables|/Game/Blueprints/Dialogue/DialogueManager.DialogueManager_C|GetNpc3Dialogues _dialoguemanager)))
    (:4
      (Variables|Default|SetNpcDialogues (Variables|/Game/Blueprints/Dialogue/DialogueManager.DialogueManager_C|GetNpc4Dialogues _dialoguemanager))))
  (Variables|Default|SetFoundFirst false)
  (Rendering|SetRenderCustomDepth (Variables|SkeletalMeshActor|GetSkeletalMeshComponent) false)
  (Utilities|Array|Clear (Variables|Default|GetDialogue))
  (bind _asbp_game_instance (Utilities|Casting|CastToBP_GameInstance (Game|GetGameInstance)))
  (bind _currentday (Default|GetDayNumber _asbp_game_instance))
  (bind _dialogueid (Default|GetCharacterDialogueId _asbp_game_instance (Variables|Default|GetCharacterID)))
  (for _array_element (Variables|Default|GetNpcDialogues)
    (if (Math|Boolean|ANDBoolean (>= (.Id (Utilities|Struct|BreakDialogueRestrictions _array_element)) _dialogueid) (<= (.MinDay (Utilities|Struct|BreakDialogueRestrictions _array_element)) _currentday) (>= (.MaxDay (Utilities|Struct|BreakDialogueRestrictions _array_element)) _currentday) (not (Variables|Default|GetFoundFirst)))
      (Development|PrintString (Utilities|String|Append "ID: " (Utilities|String|ToString(Integer) (.Id (Utilities|Struct|BreakDialogueRestrictions _array_element))) ", Dialogy length: " (Utilities|String|ToString(Integer) (Utilities|Array|Length (.Dialogue (Utilities|Struct|BreakDialogueRestrictions _array_element)))) ", MinDay: " (Utilities|String|ToString(Integer) (.MinDay (Utilities|Struct|BreakDialogueRestrictions _array_element))) ", MaxDay:" (Utilities|String|ToString(Integer) (.MaxDay (Utilities|Struct|BreakDialogueRestrictions _array_element))) ", character dialog id: " (Utilities|String|ToString(Integer) _dialogueid) ", current day" (Utilities|String|ToString(Integer) _currentday)) true true "(R=0.000000,G=0.660000,B=1.000000,A=1.000000)" 1e+01)
      (bind _output_get (Variables|Default|SetDialogue (.Dialogue (Utilities|Struct|BreakDialogueRestrictions _array_element))))
      (Development|PrintString (Utilities|String|ToString(Text) (.Text (Utilities|Struct|BreakDialogue (Utilities|Array|Get(acopy) _output_get)))) true true "(R=0.000000,G=0.660000,B=1.000000,A=1.000000)" 2e+01)
      (Variables|Default|SetFoundFirst true)
      (Development|PrintString (Utilities|String|Append "Successfull for character: " (Utilities|String|ToString(Integer) (Variables|Default|GetCharacterID))) true true "(R=0.000000,G=0.660000,B=1.000000,A=1.000000)" 1e+01))))

(event EventBeginPlay
  (Rendering|SetVisibility (Variables|Default|GetInteractionWidget) false false)
  (bind _outactors (Actor|GetAllActorsOfClass "/Game/Blueprints/Dialogue/DialogueManager.DialogueManager_C"))
  (Variables|Default|SetDialogueManager (Utilities|Array|Get(acopy) _outactors))
  (CallFunction|LoadDialogue))

(fn ConstructionScript)